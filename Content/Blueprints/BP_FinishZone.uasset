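; BP_FinishZone is a level finish trigger that ends the level once the finished count matches the game mode's player count.
; Tick caches the Players list from GM_DefaultGameMode and writes the finished count to the PlayersToFinish text.
; CollisionBox overlaps add or remove only player character 0.
; Each entry runs CheckLevelFinish, which turns the text green and calls LevelFinished on the game mode when the counts match.
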(event OnComponentBeginOverlap(CollisionBox)
  (params (OverlappedComponent :type Primitive%20Component%20Object%20Reference) (OtherActor :type Actor%20Object%20Reference) (OtherComp :type Primitive%20Component%20Object%20Reference) (OtherBodyIndex :type Integer) (bFromSweep :type Boolean) (SweepResult :type Hit%20Result%20Structure%20%28by%20ref%29))
  (if (== OtherActor (Game|GetPlayerCharacter 0))
    (Utilities|Array|Add (Variables|Default|GetPlayersFinished) OtherActor)
    (CallFunction|CheckLevelFinish)))

(event OnComponentEndOverlap(CollisionBox)
  (params (OverlappedComponent :type Primitive%20Component%20Object%20Reference) (OtherActor :type Actor%20Object%20Reference) (OtherComp :type Primitive%20Component%20Object%20Reference) (OtherBodyIndex :type Integer))
  (bind _playersfinished (Variables|Default|GetPlayersFinished))
  (if (== OtherActor (Game|GetPlayerCharacter 0))
    (Utilities|Array|RemoveIndex _playersfinished (Utilities|Array|FindItem _playersfinished OtherActor))))

(event Custom|CheckLevelFinish
  (if (== (Utilities|Array|Length (Variables|Default|GetListOfPlayers)) (Utilities|Array|Length (Variables|Default|GetPlayersFinished)))
    (Rendering|Components|TextRender|SetTextRenderColor (Variables|Default|GetPlayersToFinish) (Math|Color|MakeColor 0 255 0))
    (bind _asgm_default_game_mode (Utilities|Casting|CastToGM_DefaultGameMode (Game|GetGameMode)))
    (Default|LevelFinished _asgm_default_game_mode)))

(event EventTick
  (params (DeltaSeconds :type Float%20%28single-precision%29))
  (bind _asgm_default_game_mode (Utilities|Casting|CastToGM_DefaultGameMode (Game|GetGameMode)))
  (Variables|Default|SetListOfPlayers (Variables|/Game/Blueprints/GM_DefaultGameMode.GM_DefaultGameMode_C|GetPlayers _asgm_default_game_mode))
  (Rendering|Components|TextRender|SetText (Variables|Default|GetPlayersToFinish) (Utilities|Text|ToText(Integer) (Utilities|Array|Length (Variables|Default|GetPlayersFinished)))))

(fn ConstructionScript)