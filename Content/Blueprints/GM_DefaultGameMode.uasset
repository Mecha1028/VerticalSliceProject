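; Game mode that spawns a BP_PlayerCharacter at every PlayerStart on BeginPlay, storing each in a Players array and using its index as PlayerID.
; Each character then gets a distinct colour, spaced evenly around the hue wheel by an inline hue-to-RGB formula, which is also saved in Colours.
; Player controller 0 possesses the first character.
; LevelFinished only prints a message.
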(event Custom|LevelFinished
  (Development|PrintString "LevelFinished"))

(event EventBeginPlay
  (bind _outactors (Actor|GetAllActorsOfClass "/Script/Engine.PlayerStart"))
  (for _array_element _outactors
    (bind _returnvalue (Game|SpawnActorfromClass "/Game/Blueprints/Player/BP_PlayerCharacter.BP_PlayerCharacter_C" (Transformation|GetActorTransform _array_element) "Undefined" "MultiplyWithRoot" 0 0))
    (bind _returnvalue_2 (Utilities|Array|Add (Variables|Default|GetPlayers) _returnvalue))
    (Variables|/Game/Blueprints/Player/BP_PlayerCharacter.BP_PlayerCharacter_C|SetPlayerID _returnvalue _returnvalue_2))
  (for _array_element_2 (Variables|Default|GetPlayers)
    (bind _output_get (Variables|/Game/Blueprints/Player/BP_PlayerCharacter.BP_PlayerCharacter_C|SetColour _array_element_2 (Math|Color|MakeColor (Math|Float|Clamp(Float) (- (Math|Float|Absolute(Float) (- (* (/ (Math|Conversions|ToFloat(Integer) (Variables|/Game/Blueprints/Player/BP_PlayerCharacter.BP_PlayerCharacter_C|GetPlayerID _array_element_2)) (Math|Conversions|ToFloat(Integer) (Utilities|Array|Length (Variables|Default|GetPlayers)))) 6.0) 3.0)) 1.0)) (Math|Float|Clamp(Float) (- 2.0 (Math|Float|Absolute(Float) (- (* (/ (Math|Conversions|ToFloat(Integer) (Variables|/Game/Blueprints/Player/BP_PlayerCharacter.BP_PlayerCharacter_C|GetPlayerID _array_element_2)) (Math|Conversions|ToFloat(Integer) (Utilities|Array|Length (Variables|Default|GetPlayers)))) 6.0) 2.0)))) (Math|Float|Clamp(Float) (- 2.0 (Math|Float|Absolute(Float) (- (* (/ (Math|Conversions|ToFloat(Integer) (Variables|/Game/Blueprints/Player/BP_PlayerCharacter.BP_PlayerCharacter_C|GetPlayerID _array_element_2)) (Math|Conversions|ToFloat(Integer) (Utilities|Array|Length (Variables|Default|GetPlayers)))) 6.0) 4.0)))))))
    (Utilities|Array|Add (Variables|Default|GetColours) _output_get))
  (Pawn|Possess (Game|GetPlayerController 0) (Utilities|Array|Get(acopy) (Variables|Default|GetPlayers))))

(fn ConstructionScript)