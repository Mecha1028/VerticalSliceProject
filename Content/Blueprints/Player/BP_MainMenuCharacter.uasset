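; BP_MainMenuCharacter is a main menu character whose Manny mesh can be tinted with a colour.
; The construction script creates dynamic material instances for the mesh's two material slots and stores them.
; SetColours applies the Colour variable to the Tint parameter of both instances, while a second custom event is left empty.
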(event Custom|SetColours
  (bind _colour (Variables|Default|GetColour))
  (Rendering|Material|SetVectorParameterValue (Variables|Default|GetMaterial1) "Tint" _colour :!class /Script/Engine.MaterialInstanceDynamic)
  (Rendering|Material|SetVectorParameterValue (Variables|Default|GetMaterial2) "Tint" _colour :!class /Script/Engine.MaterialInstanceDynamic))

(event Custom|CustomEvent)

(fn ConstructionScript
  (bind _returnvalue (Rendering|Material|CreateDynamicMaterialInstance (Variables|Character|GetMesh) 0 "/Game/Assets/ControlRig/Characters/Mannequins/Materials/Instances/Manny/MI_Manny_02.MI_Manny_02" "None" :!class /Script/Engine.PrimitiveComponent))
  (Variables|Default|SetMaterial1 _returnvalue)
  (bind _returnvalue_2 (Rendering|Material|CreateDynamicMaterialInstance (Variables|Character|GetMesh) 1 "/Game/Assets/ControlRig/Characters/Mannequins/Materials/Instances/Manny/MI_Manny_01.MI_Manny_01" "None" :!class /Script/Engine.PrimitiveComponent))
  (Variables|Default|SetMaterial2 _returnvalue_2))