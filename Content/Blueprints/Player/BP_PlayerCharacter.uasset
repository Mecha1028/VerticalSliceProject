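; Player character that detects interactable actors while possessed and tints its two mesh materials with its colour.
; Each tick, a box trace runs from the actor to InteractLocation, gated by CanInteract.
; DoOnce gates send BPI_Interact targets a pre-interact message when a hit begins and a post-interact message when it ends.
; The construction script creates the dynamic materials, which are tinted once on the first tick.
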(event Custom|SetColours
  (bind _colour (Variables|Default|GetColour))
  (Rendering|Material|SetVectorParameterValue (Variables|Default|GetMaterial1) "Tint" _colour :!class /Script/Engine.MaterialInstanceDynamic)
  (Rendering|Material|SetVectorParameterValue (Variables|Default|GetMaterial2) "Tint" _colour :!class /Script/Engine.MaterialInstanceDynamic))

(event EventTick
  (params (DeltaSeconds :type Float%20%28single-precision%29))
  (Utilities|FlowControl|Sequence
    (:then_0
      (Utilities|FlowControl|DoOnce false
        (:Completed
          (CallFunction|SetColours))))
    (:then_1
      (bind (_returnvalue _outhit) (CallFunction|InteractCheck))
      (if _returnvalue
        (Utilities|FlowControl|Sequence
          (:then_0
            (if (Utilities|DoesObjectImplementInterface (.HitActor (Collision|BreakHitResult _outhit)) "/Game/Blueprints/Interaction/BPI_Interact.BPI_Interact_C")
              (Utilities|FlowControl|DoOnce false :!label _label
                (:Completed
                  (bind _output_get (Variables|Interact|SetInteractTarget (.HitActor (Collision|BreakHitResult _outhit))))
                  (Class|BPIInteract|PreInteract(Message) _output_get)))))
          (:then_1
            (goto _label_2 Reset)))
        (else
          (Utilities|FlowControl|Sequence
            (:then_0
              (goto _label Reset))
            (:then_1
              (Utilities|FlowControl|DoOnce false :!label _label_2
                (:Completed
                  (Class|BPIInteract|PostInteract(Message) (Variables|Interact|GetInteractTarget))
                  (Variables|Interact|SetInteractTarget 0))))))))))

(event EventBeginPlay
  (Variables|Interact|SetCanInteract? false))

(event EventPossessed
  (params (NewController :type Controller%20Object%20Reference))
  (Variables|Interact|SetCanInteract? true))

(event EventUnpossessed
  (params (OldController :type Controller%20Object%20Reference))
  (Variables|Interact|SetCanInteract? false))

(fn ConstructionScript
  (bind _returnvalue (Rendering|Material|CreateDynamicMaterialInstance (Variables|Character|GetMesh) 0 "/Game/Assets/ControlRig/Characters/Mannequins/Materials/Instances/Manny/MI_Manny_02.MI_Manny_02" "None" :!class /Script/Engine.PrimitiveComponent))
  (Variables|Default|SetMaterial1 _returnvalue)
  (bind _returnvalue_2 (Rendering|Material|CreateDynamicMaterialInstance (Variables|Character|GetMesh) 1 "/Game/Assets/ControlRig/Characters/Mannequins/Materials/Instances/Manny/MI_Manny_01.MI_Manny_01" "None" :!class /Script/Engine.PrimitiveComponent))
  (Variables|Default|SetMaterial2 _returnvalue_2))

(fn InteractCheck
  (bind _interactlocation (Variables|Default|GetInteractLocation))
  (if (Variables|Interact|GetCanInteract?)
    (bind (_outhit _returnvalue) (Collision|BoxTraceByChannel (Transformation|GetActorLocation) (Transformation|GetWorldLocation _interactlocation) "32.000000,32.000000,88.000000" (Transformation|GetWorldRotation _interactlocation) "TraceTypeQuery1" false 0 "None")))
  (return _returnvalue _outhit))