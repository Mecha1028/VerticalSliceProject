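; Player controller that routes Enhanced Input to the controlled character for movement, jumping, interaction and switching between player characters.
; Movement is camera-relative, using the camera's right vector and a flattened, normalized forward vector on player character 0.
; Interact calls into the current BP_PlayerCharacter.
; Swapping possesses the next entry in the game mode's Players array with wraparound, and possession caches the pawn and its PlayerID.
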(event Input|EnhancedActionEvents|EnhancedInputActionIA_Move
  (params (ActionValue :type Vector%202D%20Structure) (ElapsedSeconds :type Float%20%28double-precision%29) (TriggeredSeconds :type Float%20%28double-precision%29) (InputAction :type Input%20Action%20Object%20Reference :default "/Game/Blueprints/Player/Input/InputActions/IA_Move.IA_Move"))
  (bind _returnvalue (Game|GetPlayerCameraManager 0))
  (bind _returnvalue_2 (Game|GetPlayerCharacter 0))
  (bind _transformcomponent (Variables|/Script/Engine.PlayerCameraManager|GetTransformComponent _returnvalue))
  (bind _returnvalue_3 (Math|Vector|GetForwardVector _transformcomponent))
  (Pawn|Input|AddMovementInput _returnvalue_2 (Math|Vector|GetRightVector _transformcomponent) (.x ActionValue) false)
  (Pawn|Input|AddMovementInput _returnvalue_2 (Math|Vector|Normalize (Math|Vector|MakeVector (.x _returnvalue_3) (.y _returnvalue_3) 0.0)) (.y ActionValue) false))

(event Input|EnhancedActionEvents|EnhancedInputActionIA_Jump
  (params (ActionValue :type Boolean) (ElapsedSeconds :type Float%20%28double-precision%29) (TriggeredSeconds :type Float%20%28double-precision%29) (InputAction :type Input%20Action%20Object%20Reference :default "/Game/Blueprints/Player/Input/InputActions/IA_Jump.IA_Jump"))
  (bind _returnvalue (Game|GetPlayerCharacter 0))
  (:Triggered
    (Character|Jump _returnvalue))
  (:Completed
    (Character|StopJumping _returnvalue)))

(event Input|EnhancedActionEvents|EnhancedInputActionIA_Interact
  (params (ActionValue :type Boolean) (ElapsedSeconds :type Float%20%28double-precision%29) (TriggeredSeconds :type Float%20%28double-precision%29) (InputAction :type Input%20Action%20Object%20Reference :default "/Game/Blueprints/Player/Input/InputActions/IA_Interact.IA_Interact"))
  (bind _asbp_player_character (Utilities|Casting|CastToBP_PlayerCharacter (Variables|Default|GetCurrentPlayer)))
  (Default|Interact _asbp_player_character))

(event Input|EnhancedActionEvents|EnhancedInputActionIA_SwapPlayer
  (params (ActionValue :type Boolean) (ElapsedSeconds :type Float%20%28double-precision%29) (TriggeredSeconds :type Float%20%28double-precision%29) (InputAction :type Input%20Action%20Object%20Reference :default "/Game/Blueprints/Player/Input/InputActions/IA_SwapPlayer.IA_SwapPlayer"))
  (bind _currentplayerid (Variables|Default|GetCurrentPlayerID))
  (bind _returnvalue (+ _currentplayerid 1))
  (bind _asgm_default_game_mode (Utilities|Casting|CastToGM_DefaultGameMode (Game|GetGameMode)))
  (if (> _returnvalue (- (Utilities|Array|Length (Variables|/Game/Blueprints/GM_DefaultGameMode.GM_DefaultGameMode_C|GetPlayers _asgm_default_game_mode)) 1))
    (Pawn|Possess (Utilities|Array|Get(acopy) (Variables|/Game/Blueprints/GM_DefaultGameMode.GM_DefaultGameMode_C|GetPlayers _asgm_default_game_mode)))
    (else
      (Pawn|Possess (Utilities|Array|Get(acopy) (Variables|/Game/Blueprints/GM_DefaultGameMode.GM_DefaultGameMode_C|GetPlayers _asgm_default_game_mode) _returnvalue)))))

(event EventPossess
  (params (PossessedPawn :type Pawn%20Object%20Reference))
  (bind _output_get (Variables|Default|SetCurrentPlayer PossessedPawn))
  (bind _asbp_player_character (Utilities|Casting|CastToBP_PlayerCharacter _output_get))
  (Variables|Default|SetCurrentPlayerID (Variables|/Game/Blueprints/Player/BP_PlayerCharacter.BP_PlayerCharacter_C|GetPlayerID _asbp_player_character)))

(fn ConstructionScript)