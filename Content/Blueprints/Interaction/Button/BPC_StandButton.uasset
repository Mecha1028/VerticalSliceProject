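; Pressure-plate style button that sends an interact message to a linked target object when an actor steps on or off it.
; The trigger overlap records the first actor to enter and ignores others until that actor leaves.
; Both press and release call the same RecieveInteractMessage on ObjectToInteract, leaving the target to handle the change.
; BeginPlay raises a script error when no target is assigned.
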(event OnComponentBeginOverlap(PressButtonTrigger)
  (params (OverlappedComponent :type Primitive%20Component%20Object%20Reference) (OtherActor :type Actor%20Object%20Reference) (OtherComp :type Primitive%20Component%20Object%20Reference) (OtherBodyIndex :type Integer) (bFromSweep :type Boolean) (SweepResult :type Hit%20Result%20Structure%20%28by%20ref%29))
  (Utilities|IsValid (Variables|Default|GetFirstToPress)
    (:Is%20Not%20Valid
      (Variables|Default|SetFirstToPress OtherActor)
      (Class|BPIInteract|RecieveInteract(Message) (Variables|Default|GetObjectToInteract)))))

(event OnComponentEndOverlap(PressButtonTrigger)
  (params (OverlappedComponent :type Primitive%20Component%20Object%20Reference) (OtherActor :type Actor%20Object%20Reference) (OtherComp :type Primitive%20Component%20Object%20Reference) (OtherBodyIndex :type Integer))
  (if (== OtherActor (Variables|Default|GetFirstToPress))
    (Variables|Default|SetFirstToPress 0)
    (Class|BPIInteract|RecieveInteract(Message) (Variables|Default|GetObjectToInteract))))

(event EventBeginPlay
  (Utilities|IsValid (Variables|Default|GetObjectToInteract)
    (:Is%20Not%20Valid
      (Utilities|Debugging|RaiseScriptError (Utilities|String|Append (Utilities|GetObjectName self) " " "Missing Interact Target")))))

(fn ConstructionScript)