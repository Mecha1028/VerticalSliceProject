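; Interactable button Blueprint that triggers a linked target object when used.
; On Interact, it plays a one-shot press animation on its skeletal mesh and sends RecieveInteractMessage to ObjectToInteract.
; BeginPlay raises a script error naming the button if no valid interact target is set.
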(event EventInteract
  (Components|Animation|PlayAnimation (Variables|Default|GetSkeletalMesh) "/Game/Assets/Models/Button/AS_ButtonPress.AS_ButtonPress" false)
  (Class|BPIInteract|RecieveInteract(Message) (Variables|Default|GetObjectToInteract)))

(event EventBeginPlay
  (Utilities|IsValid (Variables|Default|GetObjectToInteract)
    (:Is%20Not%20Valid
      (Utilities|Debugging|RaiseScriptError (Utilities|String|Append (Utilities|GetObjectName self) " " "Missing Interact Target")))))

(fn ConstructionScript)