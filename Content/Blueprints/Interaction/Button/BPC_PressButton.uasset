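; Pressable button Blueprint that plays a press animation and relays an interact message to an assigned target object.
; Interact locks further presses, plays the animation on the skeletal mesh and calls RecieveInteractMessage on ObjectToInteract.
; Tick unlocks the button whenever the mesh is not playing, so the animation length acts as the cooldown.
; BeginPlay raises a script error naming the button if no target is assigned.
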(event EventTick
  (params (DeltaSeconds :type Float%20%28single-precision%29))
  (if (not (Audio|Components|Audio|IsPlaying (Variables|Default|GetSkeletalMesh)))
    (Variables|Default|SetCanInteract? true)))

(event EventInteract
  (if (Variables|Default|GetCanInteract?)
    (Variables|Default|SetCanInteract? false)
    (Components|Animation|PlayAnimation (Variables|Default|GetSkeletalMesh) "/Game/Assets/Models/Button/PressButton/AS_PressButton.AS_PressButton" false)
    (Class|BPIInteract|RecieveInteract(Message) (Variables|Default|GetObjectToInteract))))

(event EventBeginPlay
  (Utilities|IsValid (Variables|Default|GetObjectToInteract)
    (:Is%20Not%20Valid
      (Utilities|Debugging|RaiseScriptError (Utilities|String|Append (Utilities|GetObjectName self) " " "Missing Interact Target")))))

(fn ConstructionScript)