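; BPC_ColourWall is a wall tinted to match a specific player, which that player can pass through during interaction.
; Construction creates a dynamic material, and Tick tints it with that player's colour from GM_DefaultGameMode, or white if none is assigned or valid.
; PreInteract disables collision when player character 0's PlayerID matches PlayerIDNeeded, and PostInteract restores it.
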(event EventPreInteract
  (bind _asbp_player_character (Utilities|Casting|CastToBP_PlayerCharacter (Game|GetPlayerCharacter 0)))
  (if (== (Variables|/Game/Blueprints/Player/BP_PlayerCharacter.BP_PlayerCharacter_C|GetPlayerID _asbp_player_character) (Variables|Default|GetPlayerIDNeeded))
    (Collision|SetCollisionEnabled (Variables|Default|GetCollision) "NoCollision")))

(event EventPostInteract
  (Collision|SetCollisionEnabled (Variables|Default|GetCollision) "QueryAndPhysics"))

(event EventTick
  (params (DeltaSeconds :type Float%20%28single-precision%29))
  (if (< (Variables|Default|GetPlayerIDNeeded) 0)
    (Rendering|Material|SetVectorParameterValue (Variables|Default|GetMaterial) "Tint" "(R=1.000000,G=1.000000,B=1.000000,A=1.000000)" :!class /Script/Engine.MaterialInstanceDynamic :!label _label)
    (else
      (bind _asgm_default_game_mode (Utilities|Casting|CastToGM_DefaultGameMode (Game|GetGameMode)))
      (Utilities|IsValid (Utilities|Array|Get(acopy) (Variables|/Game/Blueprints/GM_DefaultGameMode.GM_DefaultGameMode_C|GetPlayers _asgm_default_game_mode) (Variables|Default|GetPlayerIDNeeded))
        (:Is%20Valid
          (Rendering|Material|SetVectorParameterValue (Variables|Default|GetMaterial) "Tint" (Variables|/Game/Blueprints/Player/BP_PlayerCharacter.BP_PlayerCharacter_C|GetColour (Utilities|Array|Get(acopy) (Variables|/Game/Blueprints/GM_DefaultGameMode.GM_DefaultGameMode_C|GetPlayers _asgm_default_game_mode) (Variables|Default|GetPlayerIDNeeded))) :!class /Script/Engine.MaterialInstanceDynamic))
        (:Is%20Not%20Valid
          (goto _label))))))

(fn ConstructionScript
  (bind _returnvalue (Rendering|Material|CreateDynamicMaterialInstance (Variables|Default|GetWall) 0 "/Game/Assets/Materials/Environment/MI_ColourWall.MI_ColourWall" "None" :!class /Script/Engine.PrimitiveComponent))
  (Variables|Default|SetMaterial _returnvalue))