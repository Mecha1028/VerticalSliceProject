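; Interactable object maker that plays a fabrication animation and spawns an instance of a configurable class.
; On interact it animates the holo and two arm meshes, then a timer spawns the object at ObjectSpawnLocation and records it in ObjectsMade.
; At ObjectLimit it destroys the array's first entry first, but never removes that entry from the array.
; BeginPlay raises a script error when no class is set.
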(event Custom|PlayAnimations
  (Components|Animation|PlayAnimation (Variables|Default|GetSkeletalMesh1) "/Game/Assets/Models/ObjectMaker/AS_ObjectMakerHolo.AS_ObjectMakerHolo" false)
  (Components|Animation|PlayAnimation (Variables|Default|GetSkeletalMesh2) "/Game/Assets/Models/ObjectMaker/AS_ObjectMakerArmRight.AS_ObjectMakerArmRight" false)
  (Components|Animation|PlayAnimation (Variables|Default|GetSkeletalMesh3) "/Game/Assets/Models/ObjectMaker/AS_ObjectMakerArmLeft.AS_ObjectMakerArmLeft" false))

(event Custom|SpawnObject
  (bind _returnvalue (Game|SpawnActorfromClass (Variables|Default|GetObjectToMake) (Transformation|GetWorldTransform (Variables|Default|GetObjectSpawnLocation)) "Undefined" "MultiplyWithRoot" 0 0))
  (Utilities|Array|Add (Variables|Default|GetObjectsMade) _returnvalue))

(event EventBeginPlay
  (if (not (Utilities|IsValidClass (Variables|Default|GetObjectToMake)))
    (Utilities|Debugging|RaiseScriptError (Utilities|String|Append (Utilities|GetObjectName self) " " "has no object to make"))))

(event EventRecieveInteract
  (if (>= (Utilities|Array|Length (Variables|Default|GetObjectsMade)) (Variables|Default|GetObjectLimit))
    (Actor|DestroyActor (Utilities|Array|Get(acopy) (Variables|Default|GetObjectsMade))))
  (CallFunction|PlayAnimations)
  (Utilities|Time|SetTimerbyEvent (delegate Custom|SpawnObject) 1.1))

(fn ConstructionScript
  (|CallParentFunction))