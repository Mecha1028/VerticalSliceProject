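; Pickup cube that the player grabs and releases through Interact, carried with the player character's physics handle.
; Grabbing switches collision to physics-only, grabs at the center of mass, and sets the player's grab target and grabbing flag.
; While held, Tick moves the handle target to the player's InteractLocation transform.
; Releasing restores query and physics collision and clears the grabbing flags.
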(event EventInteract
  (bind _collision (Variables|Default|GetCollision))
  (if (Variables|Default|GetGrabbed?)
    (bind _asbp_player_character (Utilities|Casting|CastToBP_PlayerCharacter (Game|GetPlayerCharacter 0)))
    (Collision|SetCollisionEnabled (Variables|Default|GetCollision) "QueryAndPhysics")
    (Physics|Components|PhysicsHandle|ReleaseComponent (Variables|Default|GetPhysics%20Handle))
    (Variables|Default|SetGrabbed? false)
    (Variables|/Game/Blueprints/Player/BP_PlayerCharacter.BP_PlayerCharacter_C|SetGrabbingObject? _asbp_player_character false)
    (else
      (bind _asbp_player_character_2 (Utilities|Casting|CastToBP_PlayerCharacter (Game|GetPlayerCharacter 0)))
      (Variables|Default|SetPhysics%20Handle (Variables|/Game/Blueprints/Player/BP_PlayerCharacter.BP_PlayerCharacter_C|GetPhysicsHandle _asbp_player_character_2))
      (Variables|Default|SetInteract%20Location (Variables|/Game/Blueprints/Player/BP_PlayerCharacter.BP_PlayerCharacter_C|GetInteractLocation _asbp_player_character_2))
      (Collision|SetCollisionEnabled (Variables|Default|GetCollision) "PhysicsOnly")
      (Physics|Components|PhysicsHandle|GrabComponentatLocationwithRotation (Variables|Default|GetPhysics%20Handle) _collision "None" (Physics|GetCenterOfMass _collision "None") "0, 0, 0")
      (Variables|Default|SetGrabbed? true)
      (Variables|/Game/Blueprints/Player/BP_PlayerCharacter.BP_PlayerCharacter_C|SetGrabTarget _asbp_player_character_2 self)
      (Variables|/Game/Blueprints/Player/BP_PlayerCharacter.BP_PlayerCharacter_C|SetGrabbingObject? _asbp_player_character_2 true))))

(event EventTick
  (params (DeltaSeconds :type Float%20%28single-precision%29))
  (bind _interact_location (Variables|Default|GetInteract%20Location))
  (bind _returnvalue (Transformation|GetWorldTransform _interact_location))
  (if (Variables|Default|GetGrabbed?)
    (Class|PhysicsHandleComponent|SetTargetLocationandRotation (Variables|Default|GetPhysics%20Handle) (.location _returnvalue) (.rotation _returnvalue))))

(fn ConstructionScript
  (|CallParentFunction))