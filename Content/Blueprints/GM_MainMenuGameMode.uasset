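; Main menu game mode that shows the menu widget with cursor and UI-only input, and populates the scene with coloured characters.
; On BeginPlay it spawns a BP_MainMenuCharacter at each PlayerStart, storing it in Players with its index as PlayerID.
; Each character gets an evenly spaced rainbow colour from a hue-to-RGB formula, also saved in Colours.
; Finally, the first player controller possesses the level's BP_MainMenuCamera.
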(event EventBeginPlay
  (bind _returnvalue (Game|GetPlayerController 0))
  (bind _returnvalue_2 (UserInterface|CreateWidget "/Game/Blueprints/UI/WBP_MainMenu.WBP_MainMenu_C"))
  (UserInterface|Viewport|AddtoViewport _returnvalue_2 0)
  (Variables|/Script/Engine.PlayerController|SetbShowMouseCursor _returnvalue true)
  (Input|SetInputModeUIOnly _returnvalue 0 "DoNotLock" false)
  (bind _outactors (Actor|GetAllActorsOfClass "/Script/Engine.PlayerStart"))
  (for _array_element _outactors
    (bind _returnvalue_3 (Game|SpawnActorfromClass "/Game/Blueprints/Player/BP_MainMenuCharacter.BP_MainMenuCharacter_C" (Transformation|GetActorTransform _array_element) "Undefined" "MultiplyWithRoot" 0 0))
    (bind _returnvalue_4 (Utilities|Array|Add (Variables|Default|GetPlayers) _returnvalue_3))
    (Variables|/Game/Blueprints/Player/BP_MainMenuCharacter.BP_MainMenuCharacter_C|SetPlayerID _returnvalue_3 _returnvalue_4))
  (for _array_element_2 (Variables|Default|GetPlayers)
    (bind _output_get (Variables|/Game/Blueprints/Player/BP_MainMenuCharacter.BP_MainMenuCharacter_C|SetColour _array_element_2 (Math|Color|MakeColor (Math|Float|Clamp(Float) (- (Math|Float|Absolute(Float) (- (* (/ (Math|Conversions|ToFloat(Integer) (Variables|/Game/Blueprints/Player/BP_MainMenuCharacter.BP_MainMenuCharacter_C|GetPlayerID _array_element_2)) (Math|Conversions|ToFloat(Integer) (Utilities|Array|Length (Variables|Default|GetPlayers)))) 6.0) 3.0)) 1.0)) (Math|Float|Clamp(Float) (- 2.0 (Math|Float|Absolute(Float) (- (* (/ (Math|Conversions|ToFloat(Integer) (Variables|/Game/Blueprints/Player/BP_MainMenuCharacter.BP_MainMenuCharacter_C|GetPlayerID _array_element_2)) (Math|Conversions|ToFloat(Integer) (Utilities|Array|Length (Variables|Default|GetPlayers)))) 6.0) 2.0)))) (Math|Float|Clamp(Float) (- 2.0 (Math|Float|Absolute(Float) (- (* (/ (Math|Conversions|ToFloat(Integer) (Variables|/Game/Blueprints/Player/BP_MainMenuCharacter.BP_MainMenuCharacter_C|GetPlayerID _array_element_2)) (Math|Conversions|ToFloat(Integer) (Utilities|Array|Length (Variables|Default|GetPlayers)))) 6.0) 4.0)))))))
    (Utilities|Array|Add (Variables|Default|GetColours) _output_get))
  (bind _returnvalue_5 (Actor|GetActorOfClass "/Game/Blueprints/Player/BP_MainMenuCamera.BP_MainMenuCamera_C"))
  (Pawn|Possess (Game|GetPlayerController 0) _returnvalue_5))

(fn ConstructionScript)